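; BP_Cat is a cat enemy whose Mood stat drains over time and is shown through the colour of its Cube mesh.
; BeginPlay creates a dynamic material, and Tick lowers Mood by one per second.
; Tick also binds the threshold event every frame rather than once.
; When Mood reaches a threshold, that event sets the matching MoodColours entry on the material and prints the index and current value.
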(event `self.ReceiveBeginPlay`
  (bind _returnvalue (`PrimitiveComponent.CreateDynamicMaterialInstance` (`self.Cube`) 0 null "None"))
  (set `self.AngerColour` _returnvalue))

(event `self.ReceiveTick`
  (params (DeltaSeconds :type "Float (single-precision)"))
  (bind _returnvalue (`self.GetStatByName` "Mood"))
  (`StatComponent.ModifyStat` _returnvalue (* DeltaSeconds -1.0))
  (add `StatComponent.OnStatThresholdReached` _returnvalue (delegate `OnStatThresholdReached_Event`)))

(event `OnStatThresholdReached_Event`
  (params (ThersholdIndex :type Integer))
  (`MaterialInstanceDynamic.SetVectorParameterValue` (`self.AngerColour`) "Colour" (`|GetArrayItem` (`self.MoodColours`) ThersholdIndex))
  (`KismetSystemLibrary.PrintString` (`KismetStringLibrary.Conv_IntToString` ThersholdIndex))
  (`KismetSystemLibrary.PrintString` (`KismetStringLibrary.Conv_DoubleToString` (`StatComponent.GetCurrentValue` (`self.GetStatByName` "Mood")))))

(fn `UserConstructionScript`)