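; Actor component that tracks which realities are active for the first-person character, each identified by a collision channel.
; Set, add, remove and clear functions update the stored set and pass only the changed entries to added or removed handlers.
; These handlers make the capsule block or ignore those channels and update a material parameter collection.
; Vector parameters whose R matches a reality's stencil value get G switched to show or hide it.
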(event `RealitiesAdded`
  (params (Realities :type "Set of ECollisionChannel Enum"))
  (`self.SetCollisionToChannels` Realities "ECR_Block")
  (`self.SetMPCRealities` Realities true))

(event `RealitiesRemoved`
  (params (Realities :type "Set of ECollisionChannel Enum"))
  (`self.SetCollisionToChannels` Realities)
  (`self.SetMPCRealities` Realities))

(fn `AddRealities`
  (params (Realities :type "Set of ECollisionChannel Enum"))
  (locals (DiffAdded :type "Set of ECollisionChannel Enum"))
  (bind _valuepin (`|SetForEach` Realities)
    (:`then`
      (if (not (`BlueprintSetLibrary.Set_Contains` (`self.Realities`) _valuepin))
        (`BlueprintSetLibrary.Set_Add` (`self.Realities`) _valuepin)
        (`BlueprintSetLibrary.Set_Add` (`local.DiffAdded`) _valuepin)))
    (:`CompletedPin`
      (`self.RealitiesAdded` (`local.DiffAdded`)))))

(fn `ClearRealities`
  (locals (DiffCleared :type "Set of ECollisionChannel Enum"))
  (bind _realities (`self.Realities`))
  (set `local.DiffCleared` _realities)
  (`BlueprintSetLibrary.Set_Clear` _realities)
  (`self.RealitiesRemoved` (`local.DiffCleared`)))

(fn `GetRealities`
  (returns (Channels :type "Set of ECollisionChannel Enum"))
  (return (`self.Realities`)))

(fn `HasReality`
  (params (Reality :type "ECollisionChannel Enum" :default "ECC_WorldStatic"))
  (returns (Bool :type Boolean))
  (return (`BlueprintSetLibrary.Set_Contains` (`self.Realities`) Reality)))

(fn `RemoveRealities`
  (params (Realities :type "Set of ECollisionChannel Enum"))
  (locals (DiffRemoved :type "Set of ECollisionChannel Enum"))
  (bind _valuepin (`|SetForEach` Realities)
    (:`then`
      (bind _returnvalue (`BlueprintSetLibrary.Set_Remove` (`self.Realities`) _valuepin))
      (if _returnvalue
        (`BlueprintSetLibrary.Set_Add` (`local.DiffRemoved`) _valuepin)))
    (:`CompletedPin`
      (`self.RealitiesRemoved` (`local.DiffRemoved`)))))

(fn `SetCollisionToChannels`
  (params (Channels :type "Set of ECollisionChannel Enum") (Response :type "ECollisionResponse Enum" :default "ECR_Ignore"))
  (bind _asbp_first_person_character (cast `/Game/FirstPerson/Blueprints/BP_FirstPersonCharacter` (`self.GetOwner`)))
  (bind _valuepin (`|SetForEach` Channels)
    (:`then`
      (`PrimitiveComponent.SetCollisionResponseToChannel` (`Character.CapsuleComponent` _asbp_first_person_character) _valuepin Response))))

(fn `SetMPCRealities`
  (params (Realities :type "Set of ECollisionChannel Enum") (IsVisible :type Boolean))
  (locals (RealityStencils :type "Set of Float (double-precision)"))
  (bind _collection (`self.Collection`))
  (bind _valuepin (`|SetForEach` Realities)
    (:`then`
      (bind (_stencilvalue _isreality) (`/Game/RealitySystem/StencilDepthHelper/BPFL_RealityStencilHelper.StencilDepth` _valuepin))
      (if _isreality
        (`BlueprintSetLibrary.Set_Add` (`local.RealityStencils`) (`KismetMathLibrary.Conv_IntToDouble` _stencilvalue))))
    (:`CompletedPin`
      (for _array_element (`MaterialParameterCollection.GetVectorParameterNames` _collection)
        (bind _returnvalue (`KismetMaterialLibrary.GetVectorParameterValue` _collection _array_element))
        (if (`BlueprintSetLibrary.Set_Contains` (`local.RealityStencils`) (break `LinearColor` _returnvalue))
          (`KismetMaterialLibrary.SetVectorParameterValue` _collection _array_element (make `LinearColor` (break `LinearColor` _returnvalue) (`KismetMathLibrary.SelectFloat` 1.0 0.0 (`local.IsVisible`)) (`.B` (break `LinearColor` _returnvalue)) (`.A` (break `LinearColor` _returnvalue)))))))))

(fn `SetRealities`
  (params (Realities :type "Set of ECollisionChannel Enum"))
  (locals (DiffAdded :type "Set of ECollisionChannel Enum") (DiffRemoved :type "Set of ECollisionChannel Enum"))
  (bind _valuepin (`|SetForEach` Realities)
    (:`then`
      (if (not (`self.HasReality` _valuepin))
        (`BlueprintSetLibrary.Set_Add` (`local.DiffAdded`) _valuepin)))
    (:`CompletedPin`
      (bind _valuepin_2 (`|SetForEach` (`self.Realities`))
        (:`then`
          (if (not (`BlueprintSetLibrary.Set_Contains` Realities _valuepin_2))
            (`BlueprintSetLibrary.Set_Add` (`local.DiffRemoved`) _valuepin_2)))
        (:`CompletedPin`
          (set `self.Realities` Realities)
          (`self.RealitiesAdded` (`local.DiffAdded`))
          (`self.RealitiesRemoved` (`local.DiffRemoved`)))))))