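; Actor component that assigns its owning actor to a Reality, controlling how it renders and what it collides with.
; On BeginPlay and on SetReality, it sets custom depth, stencil value and a RealityStencil material parameter on the owner's static meshes from that Reality.
; Physics-enabled primitives switch to the Reality's object channel, blocking only that channel and a default block list.
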(event `self.ReceiveBeginPlay`
  (`self.InitVisibility`)
  (`self.InitCollision`))

(fn `GetReality`
  (returns (Reality :type "ECollisionChannel Enum"))
  (return (`self.Reality`)))

(fn `InitCollision`
  (locals (CollisionType :type "ECollisionEnabled Enum"))
  (bind _reality (`self.Reality`))
  (for _array_element (`Actor.K2_GetComponentsByClass` (`self.GetOwner`) "/Script/Engine.PrimitiveComponent")
    (switch `ECollisionEnabled` (`PrimitiveComponent.GetCollisionEnabled` _array_element)
      (:`PhysicsOnly`
        _)
      (:`QueryAndPhysics`
        _))
    (`PrimitiveComponent.SetCollisionObjectType` _array_element _reality)
    (`PrimitiveComponent.SetCollisionResponseToAllChannels` _array_element "ECR_Ignore")
    (for _array_element_2 (`self.DefaultBlockList`)
      (`PrimitiveComponent.SetCollisionResponseToChannel` _array_element _array_element_2 "ECR_Block"))
    (`PrimitiveComponent.SetCollisionResponseToChannel` _array_element _reality "ECR_Block")))

(fn `InitVisibility`
  (locals (IsVisible :type Boolean))
  (bind (_stencilvalue _isreality) (`/Game/RealitySystem/StencilDepthHelper/BPFL_RealityStencilHelper.StencilDepth` (`self.Reality`)))
  (for _array_element (`Actor.K2_GetComponentsByClass` (`self.GetOwner`) "/Script/Engine.StaticMeshComponent")
    (`PrimitiveComponent.SetRenderCustomDepth` _array_element _isreality)
    (`PrimitiveComponent.SetCustomDepthStencilValue` _array_element _stencilvalue)
    (`MeshComponent.SetScalarParameterValueOnMaterials` _array_element "RealityStencil" (`KismetMathLibrary.Conv_IntToDouble` _stencilvalue))))

(fn `SetReality`
  (params (Reality :type "ECollisionChannel Enum" :default "ECC_WorldStatic"))
  (set `self.Reality` Reality)
  (`self.InitCollision`)
  (`self.InitVisibility`))