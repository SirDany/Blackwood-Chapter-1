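; Poolable window between realities that lets the first-person player see and step through to another reality, with one assigned per side.
; Front and back collisions track entry direction, adding that side's reality to the player's RealityManager, then setting it on crossing or removing it on backing out.
; Each tick, a camera-facing dot test picks the plane's custom stencil value, offset via MPC_ActiveRealities for realities, and hides inactive windows.
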(event `self.ReceiveTick`
  (params (DeltaSeconds :type "Float (single-precision)"))
  (`self.UpdatePlaneStencil`))

(event `self.BackCollision.OnComponentBeginOverlap`
  (params (OverlappedComponent :type "PrimitiveComponent Object Reference") (OtherActor :type "Actor Object Reference") (OtherComp :type "PrimitiveComponent Object Reference") (OtherBodyIndex :type Integer) (bFromSweep :type Boolean) (SweepResult :type "HitResult Structure (by ref)"))
  (bind _backtofrontreality (`self.BackToFrontReality`))
  (bind _asbp_first_person_character (cast `/Game/FirstPerson/Blueprints/BP_FirstPersonCharacter` OtherActor))
  (if (and (`self.IsActive`) (`|EnumEquality` (`self.EntryDirection`) "NewEnumerator2") (`.IsReality` (`/Game/RealitySystem/StencilDepthHelper/BPFL_RealityStencilHelper.StencilDepth` _backtofrontreality)))
    (set `self.EntryDirection` "NewEnumerator1")
    (`/Game/RealitySystem/AC_RealityManager.AddRealities` (`/Game/FirstPerson/Blueprints/BP_FirstPersonCharacter.AC_RealityManager` _asbp_first_person_character) (`|MakeSet` _backtofrontreality))))

(event `self.BackCollision.OnComponentEndOverlap`
  (params (OverlappedComponent :type "PrimitiveComponent Object Reference") (OtherActor :type "Actor Object Reference") (OtherComp :type "PrimitiveComponent Object Reference") (OtherBodyIndex :type Integer))
  (bind _backtofrontreality (`self.BackToFrontReality`))
  (bind _set (`|MakeSet` _backtofrontreality))
  (bind _asbp_first_person_character (cast `/Game/FirstPerson/Blueprints/BP_FirstPersonCharacter` OtherActor))
  (if (and (`.IsReality` (`/Game/RealitySystem/StencilDepthHelper/BPFL_RealityStencilHelper.StencilDepth` _backtofrontreality)) (`|EnumEquality` (`self.EntryDirection`) "NewEnumerator1"))
    (if (`PrimitiveComponent.IsOverlappingActor` (`self.FrontCollision`) _asbp_first_person_character)
      (bind _ac_realitymanager (`/Game/FirstPerson/Blueprints/BP_FirstPersonCharacter.AC_RealityManager` _asbp_first_person_character))
      (`/Game/RealitySystem/AC_RealityManager.SetRealities` _ac_realitymanager _set)
      (set `self.EntryDirection` "NewEnumerator2")
      (`self.SteppedThroughBack`)
      (else
        (`/Game/RealitySystem/AC_RealityManager.RemoveRealities` _ac_realitymanager _set)
        (set `self.EntryDirection` "NewEnumerator2")))))

(event `self.FrontCollision.OnComponentBeginOverlap`
  (params (OverlappedComponent :type "PrimitiveComponent Object Reference") (OtherActor :type "Actor Object Reference") (OtherComp :type "PrimitiveComponent Object Reference") (OtherBodyIndex :type Integer) (bFromSweep :type Boolean) (SweepResult :type "HitResult Structure (by ref)"))
  (bind _fronttobackreality (`self.FrontToBackReality`))
  (bind _asbp_first_person_character (cast `/Game/FirstPerson/Blueprints/BP_FirstPersonCharacter` OtherActor))
  (if (and (`self.IsActive`) (`|EnumEquality` (`self.EntryDirection`) "NewEnumerator2") (`.IsReality` (`/Game/RealitySystem/StencilDepthHelper/BPFL_RealityStencilHelper.StencilDepth` _fronttobackreality)))
    (set `self.EntryDirection` "NewEnumerator0")
    (`/Game/RealitySystem/AC_RealityManager.AddRealities` (`/Game/FirstPerson/Blueprints/BP_FirstPersonCharacter.AC_RealityManager` _asbp_first_person_character) (`|MakeSet` _fronttobackreality))))

(event `self.FrontCollision.OnComponentEndOverlap`
  (params (OverlappedComponent :type "PrimitiveComponent Object Reference") (OtherActor :type "Actor Object Reference") (OtherComp :type "PrimitiveComponent Object Reference") (OtherBodyIndex :type Integer))
  (bind _fronttobackreality (`self.FrontToBackReality`))
  (bind _set (`|MakeSet` _fronttobackreality))
  (bind _asbp_first_person_character (cast `/Game/FirstPerson/Blueprints/BP_FirstPersonCharacter` OtherActor))
  (if (and (`.IsReality` (`/Game/RealitySystem/StencilDepthHelper/BPFL_RealityStencilHelper.StencilDepth` _fronttobackreality)) (`|EnumEquality` (`self.EntryDirection`) "NewEnumerator0"))
    (if (`PrimitiveComponent.IsOverlappingActor` (`self.BackCollision`) _asbp_first_person_character)
      (bind _ac_realitymanager (`/Game/FirstPerson/Blueprints/BP_FirstPersonCharacter.AC_RealityManager` _asbp_first_person_character))
      (`/Game/RealitySystem/AC_RealityManager.SetRealities` _ac_realitymanager _set)
      (set `self.EntryDirection` "NewEnumerator2")
      (`self.SteppedThroughFront`)
      (else
        (`/Game/RealitySystem/AC_RealityManager.RemoveRealities` _ac_realitymanager _set)
        (set `self.EntryDirection` "NewEnumerator2")))))

(fn `BackwardsVector`
  (returns (Backwards :type "Vector Structure"))
  (bind _forward (`self.ForwardVector`))
  (return (`KismetMathLibrary.NegateVector` _forward)))

(fn `ForwardVector`
  (returns (Forward :type "Vector Structure"))
  (return (`SceneComponent.GetForwardVector` (`self.Forward`))))

(fn `LookingAtFront`
  (returns (ReturnValue :type Boolean))
  (return (> (`KismetMathLibrary.Dot_VectorVector` (`KismetMathLibrary.Normal` (- (`PlayerCameraManager.GetCameraLocation` (`GameplayStatics.GetPlayerCameraManager` 0)) (`SceneComponent.K2_GetComponentLocation` (`self.RealityPlane`)))) (`SceneComponent.GetForwardVector` (`self.Forward`))) 0.0)))

(fn `ReturnToPool`
  (set `self.FrontToBackReality` "ECC_WorldStatic")
  (set `self.BackToFrontReality` "ECC_WorldStatic")
  (set `self.EntryDirection` "NewEnumerator2")
  (set `self.IsActive` false)
  (`parent.ReturnToPool`))

(fn `SetFrameMaterial`
  (params (Material :type "MaterialInstance Object Reference"))
  (set `self.FrameMaterial` Material)
  (for _array_element (`|MakeArray` (`self.Bottom`) (`self.Left`) (`self.Right`) (`self.Top`))
    (`PrimitiveComponent.SetMaterial` _array_element 0 (`self.FrameMaterial`))))

(fn `UpdatePlaneStencil`
  (bind (_stencilvalue _isreality) (`/Game/RealitySystem/StencilDepthHelper/BPFL_RealityStencilHelper.StencilDepth` (select `bool` (`self.LookingAtFront`) :`false` (`self.BackToFrontReality`) :`true` (`self.FrontToBackReality`))))
  (bind _returnvalue (`KismetMaterialLibrary.GetScalarParameterValue` "/Game/RealitySystem/Materials/MPC_ActiveRealities.MPC_ActiveRealities" "WindowStencilOffset"))
  (`PrimitiveComponent.SetCustomDepthStencilValue` (`self.RealityPlane`) (`KismetMathLibrary.SelectInt` (`KismetMathLibrary.FTrunc` (+ _returnvalue _stencilvalue)) _stencilvalue _isreality))
  (`self.SetActorHiddenInGame` (not (`self.IsActive`))))

(fn `UserConstructionScript`
  (bind _framematerial (`self.FrameMaterial`))
  (`/Engine/EditorBlueprintResources/StandardMacros.IsValid` _framematerial
    (:`Is Valid`
      (`self.SetFrameMaterial` _framematerial))))