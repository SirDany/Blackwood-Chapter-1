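; A two-sided framed window actor that shows a different reality from each side and lets the first-person character step through into it.
; Each Tick it sets the plane's custom depth stencil from the side the camera faces, offsetting reality values by a material parameter collection scalar.
; Front and back collisions track entry direction, adding that side's reality on entry, then setting it on crossing or removing it on retreat.
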(event `self.ReceiveTick`
  (params (DeltaSeconds :type "Float (single-precision)"))
  (`self.UpdatePlaneStencil`))

(event `self.BackCollision.OnComponentBeginOverlap`
  (params (OverlappedComponent :type "PrimitiveComponent Object Reference") (OtherActor :type "Actor Object Reference") (OtherComp :type "PrimitiveComponent Object Reference") (OtherBodyIndex :type Integer) (bFromSweep :type Boolean) (SweepResult :type "HitResult Structure (by ref)"))
  (bind _backtofrontrealities (`self.BackToFrontRealities`))
  (bind _asbp_first_person_character (cast `/Game/FirstPerson/Blueprints/BP_FirstPersonCharacter` OtherActor))
  (if (and (`|EnumEquality` (`self.EntryDirection`) "NewEnumerator2") (`.IsReality` (`/Game/RealitySystem/StencilDepthHelper/BPFL_RealityStencilHelper.StencilDepth` _backtofrontrealities)))
    (set `self.EntryDirection` "NewEnumerator1")
    (`/Game/RealitySystem/AC_RealityManager.AddRealities` (`/Game/FirstPerson/Blueprints/BP_FirstPersonCharacter.AC_RealityManager` _asbp_first_person_character) (`|MakeSet` _backtofrontrealities))))

(event `self.BackCollision.OnComponentEndOverlap`
  (params (OverlappedComponent :type "PrimitiveComponent Object Reference") (OtherActor :type "Actor Object Reference") (OtherComp :type "PrimitiveComponent Object Reference") (OtherBodyIndex :type Integer))
  (bind _backtofrontrealities (`self.BackToFrontRealities`))
  (bind _set (`|MakeSet` _backtofrontrealities))
  (bind _asbp_first_person_character (cast `/Game/FirstPerson/Blueprints/BP_FirstPersonCharacter` OtherActor))
  (if (and (`.IsReality` (`/Game/RealitySystem/StencilDepthHelper/BPFL_RealityStencilHelper.StencilDepth` _backtofrontrealities)) (`|EnumEquality` (`self.EntryDirection`) "NewEnumerator1"))
    (if (`PrimitiveComponent.IsOverlappingActor` (`self.FrontCollision`) _asbp_first_person_character)
      (bind _ac_realitymanager (`/Game/FirstPerson/Blueprints/BP_FirstPersonCharacter.AC_RealityManager` _asbp_first_person_character))
      (`/Game/RealitySystem/AC_RealityManager.SetRealities` _ac_realitymanager _set)
      (set `self.EntryDirection` "NewEnumerator2")
      (`self.SteppedThroughBack`)
      (else
        (`/Game/RealitySystem/AC_RealityManager.RemoveRealities` _ac_realitymanager _set)
        (set `self.EntryDirection` "NewEnumerator2")))))

(event `self.FrontCollision.OnComponentBeginOverlap`
  (params (OverlappedComponent :type "PrimitiveComponent Object Reference") (OtherActor :type "Actor Object Reference") (OtherComp :type "PrimitiveComponent Object Reference") (OtherBodyIndex :type Integer) (bFromSweep :type Boolean) (SweepResult :type "HitResult Structure (by ref)"))
  (bind _fronttobackrealities (`self.FrontToBackRealities`))
  (bind _asbp_first_person_character (cast `/Game/FirstPerson/Blueprints/BP_FirstPersonCharacter` OtherActor))
  (if (and (`|EnumEquality` (`self.EntryDirection`) "NewEnumerator2") (`.IsReality` (`/Game/RealitySystem/StencilDepthHelper/BPFL_RealityStencilHelper.StencilDepth` _fronttobackrealities)))
    (set `self.EntryDirection` "NewEnumerator0")
    (`/Game/RealitySystem/AC_RealityManager.AddRealities` (`/Game/FirstPerson/Blueprints/BP_FirstPersonCharacter.AC_RealityManager` _asbp_first_person_character) (`|MakeSet` _fronttobackrealities))))

(event `self.FrontCollision.OnComponentEndOverlap`
  (params (OverlappedComponent :type "PrimitiveComponent Object Reference") (OtherActor :type "Actor Object Reference") (OtherComp :type "PrimitiveComponent Object Reference") (OtherBodyIndex :type Integer))
  (bind _fronttobackrealities (`self.FrontToBackRealities`))
  (bind _set (`|MakeSet` _fronttobackrealities))
  (bind _asbp_first_person_character (cast `/Game/FirstPerson/Blueprints/BP_FirstPersonCharacter` OtherActor))
  (if (and (`.IsReality` (`/Game/RealitySystem/StencilDepthHelper/BPFL_RealityStencilHelper.StencilDepth` _fronttobackrealities)) (`|EnumEquality` (`self.EntryDirection`) "NewEnumerator0"))
    (if (`PrimitiveComponent.IsOverlappingActor` (`self.BackCollision`) _asbp_first_person_character)
      (bind _ac_realitymanager (`/Game/FirstPerson/Blueprints/BP_FirstPersonCharacter.AC_RealityManager` _asbp_first_person_character))
      (`/Game/RealitySystem/AC_RealityManager.SetRealities` _ac_realitymanager _set)
      (set `self.EntryDirection` "NewEnumerator2")
      (`self.SteppedThroughFront`)
      (else
        (`/Game/RealitySystem/AC_RealityManager.RemoveRealities` _ac_realitymanager _set)
        (set `self.EntryDirection` "NewEnumerator2")))))

(fn `BackwardsVector`
  (returns (Backwards :type "Vector Structure"))
  (return (`KismetMathLibrary.NegateVector` (`SceneComponent.GetForwardVector` (`self.Forward`)))))

(fn `LookingAtFront`
  (returns (ReturnValue :type Boolean))
  (return (> (`KismetMathLibrary.Dot_VectorVector` (`KismetMathLibrary.Normal` (- (`PlayerCameraManager.GetCameraLocation` (`GameplayStatics.GetPlayerCameraManager` 0)) (`SceneComponent.K2_GetComponentLocation` (`self.RealityPlane`)))) (`SceneComponent.GetForwardVector` (`self.Forward`))) 0.0)))

(fn `UpdatePlaneStencil`
  (bind (_stencilvalue _isreality) (`/Game/RealitySystem/StencilDepthHelper/BPFL_RealityStencilHelper.StencilDepth` (select `bool` (`self.LookingAtFront`) :`false` (`self.BackToFrontRealities`) :`true` (`self.FrontToBackRealities`))))
  (bind _returnvalue (`KismetMaterialLibrary.GetScalarParameterValue` "/Game/RealitySystem/Materials/MPC_ActiveRealities.MPC_ActiveRealities" "WindowStencilOffset"))
  (`PrimitiveComponent.SetCustomDepthStencilValue` (`self.RealityPlane`) (`KismetMathLibrary.SelectInt` (`KismetMathLibrary.FTrunc` (+ _returnvalue _stencilvalue)) _stencilvalue _isreality)))

(fn `UserConstructionScript`
  (`/Engine/EditorBlueprintResources/StandardMacros.IsValid` (`self.FrameMaterial`)
    (:`Is Valid`
      (for _array_element (`|MakeArray` (`self.Bottom`) (`self.Left`) (`self.Right`) (`self.Top`))
        (`PrimitiveComponent.SetMaterial` _array_element 0 (`self.FrameMaterial`))))))