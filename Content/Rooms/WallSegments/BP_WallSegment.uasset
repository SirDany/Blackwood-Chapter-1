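; BP_WallSegment is a poolable room wall piece that scales its body to a given size and can host a single door.
; It counts as blocked when it holds a door or is flagged externally, shown through a material parameter on the debug-visible body.
; PlaceDoor puts a door at floor center of an unblocked segment, deriving yaw from the inward vector and the door's forward, supplied by I_Directional when implemented.
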(event `self.ReceiveBeginPlay`
  (`self.Init` (`self.Size`)))

(fn `DestroyDoor`
  (bind _door (`self.Door`))
  (`/Engine/EditorBlueprintResources/StandardMacros.IsValid` _door
    (:`Is Valid`
      (`self.K2_DestroyActor` _door)
      (`self.UpdateDebuggingMaterial`))))

(fn `ForwardVector`
  (returns (Forward :type "Vector Structure"))
  (return (`SceneComponent.GetForwardVector` (`self.Inward`))))

(fn `GetDoor`
  (returns (Door :type "/Game/Rooms/BP_Door Object Reference"))
  (return (`self.Door`)))

(fn `HandleDebugging`
  (`SceneComponent.SetHiddenInGame` (`self.Inward`) (not (`self.Debugging`)) false)
  (`SceneComponent.SetVisibility` (`self.Body`) (`self.Debugging`) false)
  (`self.UpdateDebuggingMaterial`))

(fn `Init`
  (params (Size :type "Vector Structure"))
  (bind _body (`self.Body`))
  (bind (_size_x _size_y _size_z) (`KismetMathLibrary.BreakVector` (`self.Size`)))
  (bind (_relativelocation_x _relativelocation_y) (`KismetMathLibrary.BreakVector` (`SceneComponent.RelativeLocation` _body)))
  (bind _output_get (set `self.Size` Size))
  (`SceneComponent.SetWorldScale3D` (`self.Body`) (/ _output_get 100.0))
  (`SceneComponent.K2_SetRelativeLocation` _body (`KismetMathLibrary.MakeVector` _relativelocation_x _relativelocation_y (/ _size_z 2.0)) false false)
  (`self.HandleDebugging`))

(fn `IsBlocked`
  (returns (Blocked :type Boolean))
  (return (or (`KismetSystemLibrary.IsValid` (`self.Door`)) (`self.IsBlockedExternal`))))

(fn `PlaceDoor`
  (params (Door :type "/Game/Rooms/BP_Door Object Reference"))
  (if (not (`self.IsBlocked`))
    (bind _forward (message `/Game/Utils/I_Directional.ForwardVector` Door))
    (bind _forward_2 (`self.ForwardVector`))
    (`self.K2_SetActorTransform` Door (`KismetMathLibrary.MakeTransform` (`KismetMathLibrary.TransformLocation` (`SceneComponent.K2_GetComponentToWorld` (`self.DefaultSceneRoot`)) (`self.PlacementCoordinates` "NewEnumerator0" "NewEnumerator4")) (`KismetMathLibrary.MakeRotator` 0.0 0.0 (`/Game/Utils/BPFL_Utils.CalcYawFromTo` _forward_2 (`KismetMathLibrary.SelectVector` _forward (`self.GetActorForwardVector` Door) (`KismetSystemLibrary.DoesImplementInterface` Door "/Game/Utils/I_Directional.I_Directional_C"))))) false false)
    (set `self.Door` Door)
    (`self.UpdateDebuggingMaterial`)))

(fn `PlacementCoordinates`
  (params (Horizontal :type "/Game/Rooms/WallSegments/EN_WallSegmentHorizontalAlignment Enum" :default "NewEnumerator0") (Vertical :type "/Game/Rooms/WallSegments/EN_WallSegmentVerticalAlignment Enum" :default "NewEnumerator0"))
  (returns (Location :type "Vector Structure"))
  (bind _size_x (`KismetMathLibrary.BreakVector` (`self.Size`)))
  (bind (_size_x_2 _size_y _size_z) (`KismetMathLibrary.BreakVector` (`self.Size`)))
  (bind _returnvalue (/ _size_z 6.0))
  (bind _returnvalue_2 (/ _size_x 6.0))
  (return (`KismetMathLibrary.MakeVector` (select `/Game/Rooms/WallSegments/EN_WallSegmentHorizontalAlignment` Horizontal :`NewEnumerator1` (* _returnvalue_2 -1.0) :`NewEnumerator2` _returnvalue_2) 0.0 (select `/Game/Rooms/WallSegments/EN_WallSegmentVerticalAlignment` Vertical :`NewEnumerator0` (/ _size_z 2.0) :`NewEnumerator1` (- _size_z _returnvalue) :`NewEnumerator2` _returnvalue :`NewEnumerator3` _size_z))))

(fn `RemoveDoor`
  (set `self.Door` null)
  (`self.UpdateDebuggingMaterial`))

(fn `ReturnToPool`
  (set `self.RelativeLoaction` (0.0 0.0 0.0))
  (set `self.IsBlockedExternal` false)
  (`self.RemoveDoor`)
  (`parent.ReturnToPool`))

(fn `SetBlocked`
  (params (IsBlocked :type Boolean))
  (set `self.IsBlockedExternal` IsBlocked)
  (`self.UpdateDebuggingMaterial`))

(fn `SetDoor`
  (params (Door :type "/Game/Rooms/BP_Door Object Reference"))
  (set `self.Door` Door)
  (`self.UpdateDebuggingMaterial`))

(fn `UpdateDebuggingMaterial`
  (`MeshComponent.SetScalarParameterValueOnMaterials` (`self.Body`) "IsBlocked" (`KismetMathLibrary.Conv_BoolToDouble` (`self.IsBlocked`))))

(fn `UserConstructionScript`)