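; BP_Door is a pooled door actor that links a front room and a back room.
; It binds the front and back step-through events and calls SteppedThrough with the entered and exited rooms.
; Toggle switches collision on the actor and four frame sides, while RealityPlane collision stays disabled there and in SetInUse.
; RemoveRoom clears matching room references, and ReturnToPool clears both before running parent logic.
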(event `self.ReceiveBeginPlay`
  (`parent.ReceiveBeginPlay`)
  (add `self.SteppedThroughFront` (delegate `EnteredBackRoom`))
  (add `self.SteppedThroughBack` (delegate `EnteredFrontRoom`)))

(event `EnteredBackRoom`
  (`self.SteppedThrough` (`self.BackRoom`) (`self.FrontRoom`)))

(event `EnteredFrontRoom`
  (`self.SteppedThrough` (`self.FrontRoom`) (`self.BackRoom`)))

(fn `RemoveRoom`
  (params (Room :type "/Game/Rooms/BP_Room Object Reference"))
  (`|ExecutionSequence`
    (:`then_0`
      (if (== (`self.FrontRoom`) Room)
        (set `self.FrontRoom` null)))
    (:`then_1`
      (if (== Room (`self.BackRoom`))
        (set `self.BackRoom` null)))))

(fn `ReturnToPool`
  (set `self.FrontRoom` null)
  (set `self.BackRoom` null)
  (`parent.ReturnToPool`))

(fn `SetInUse`
  (params (InUse :type Boolean))
  (`parent.SetInUse` InUse)
  (`PrimitiveComponent.SetCollisionEnabled` (`self.RealityPlane`) "NoCollision"))

(fn `Toggle`
  (params (IsActive :type Boolean))
  (bind _returnvalue (select `bool` IsActive :`false` "NoCollision" :`true` "QueryAndPhysics" :!type "ECollisionEnabled Enum"))
  (bind _output_get (set `self.IsActive` IsActive))
  (`self.SetActorEnableCollision` _output_get)
  (`PrimitiveComponent.SetCollisionEnabled` (`self.RealityPlane`) "NoCollision")
  (`|ExecutionSequence`
    (:`then_0`
      (`PrimitiveComponent.SetCollisionEnabled` (`self.Bottom`) _returnvalue))
    (:`then_1`
      (`PrimitiveComponent.SetCollisionEnabled` (`self.Left`) _returnvalue))
    (:`then_2`
      (`PrimitiveComponent.SetCollisionEnabled` (`self.Right`) _returnvalue))
    (:`then_3`
      (`PrimitiveComponent.SetCollisionEnabled` (`self.Top`) _returnvalue))))

(fn `UserConstructionScript`
  (`parent.UserConstructionScript`))