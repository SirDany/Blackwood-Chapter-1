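; Room manager that grows a procedural maze of pooled BP_Rooms around the player as doors are stepped through.
; Entering a room spawns its missing neighbours, flipping doors whose previous room was removed, and switches active doors.
; A capped backtracking stack recycles the oldest room and its off-path neighbours.
; Doors get cycled realities, and exit counts use cumulative weights from a DataTable, which also help size the pool.
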(event Custom|InitialEntry
  (params (Entered :type BP%20Room%20Object%20Reference) (Exited :type BP%20Room%20Object%20Reference))
  (EventDispatchers|UnbindEventfromSteppedThrough (Variables|Default|GetFirstEntry) (delegate Custom|InitialEntry))
  (Default|CallMazeEntered))

(event Custom|RoomEntered
  (params (Entered :type BP%20Room%20Object%20Reference) (Exited :type BP%20Room%20Object%20Reference))
  (Private|UpdateBacktrackingOrder Entered)
  (CallFunction|SpawnMissingNeighbours Entered)
  ;[0.15 0.15 0.15 0.5] Important: First deactive, then activate -> entry door is shared by both
  (Utilities|IsValid Exited
    (:Is%20Valid
      (Default|ToggleDoors Exited false))
    (:Is%20Not%20Valid
      _))
  (Default|ToggleDoors Entered true))

(event EventBeginPlay
  (bind _firstentry (Variables|Default|GetFirstEntry))
  (Private|Helper|BuildExitDoorWeightsLookup)
  (Private|InitObjectPools)
  (Utilities|IsValid _firstentry
    (:Is%20Valid
      (Private|SpawnRoom _firstentry)
      (EventDispatchers|BindEventtoSteppedThrough _firstentry (delegate Custom|InitialEntry)))))

(fn ConstructionScript)

(fn SpawnRoom
  (params (Entry :type BP%20Door%20Object%20Reference))
  (bind _pooledactor (Default|SpawnfromPool (Variables|Default|GetAC_RoomsPool)))
  (bind _asbp_room (Utilities|Casting|CastToBP_Room _pooledactor))
  (Default|BuildRoom _asbp_room Entry)
  (Default|SetReality (Variables|/Game/Rooms/BP_Room.BP_Room_C|GetAC_RealityObject _asbp_room) (Variables|/Game/RealitySystem/RealityWindow/BP_RealityWindow.BP_RealityWindow_C|GetFrontToBackReality Entry))
  (Utilities|Map|Add (Variables|Default|GetRooms) (Variables|/Game/Rooms/BP_Room.BP_Room_C|GetRoomID _asbp_room) _asbp_room)
  (for _array_element (Default|Doors _asbp_room)
    (Utilities|FlowControl|Sequence
      (:then_0
        ;[0.15 0.15 0.15 0.5] Bind to step through events
        (if (not (Utilities|Set|Contains (Variables|Private|GetBoundDoors) _array_element))
          (EventDispatchers|BindEventtoSteppedThrough _array_element (EventDispatchers|CreateEvent :!event Custom|RoomEntered))
          (Utilities|Set|Add (Variables|Private|GetBoundDoors) _array_element)))
      (:then_1
        ;[0.15 0.15 0.15 0.5] Assign realities to doors
        (if (not (Utilities|Array|ContainsItem (Variables|Private|GetRoomRealities) (Variables|/Game/RealitySystem/RealityWindow/BP_RealityWindow.BP_RealityWindow_C|GetFrontToBackReality _array_element)))
          (Variables|/Game/RealitySystem/RealityWindow/BP_RealityWindow.BP_RealityWindow_C|SetFrontToBackReality _array_element (Private|NextRoomReality))))
      (:then_2
        (if (not (Utilities|Array|ContainsItem (Variables|Private|GetRoomRealities) (Variables|/Game/RealitySystem/RealityWindow/BP_RealityWindow.BP_RealityWindow_C|GetBackToFrontReality _array_element)))
          (Variables|/Game/RealitySystem/RealityWindow/BP_RealityWindow.BP_RealityWindow_C|SetBackToFrontReality _array_element (Variables|/Game/RealitySystem/RealityWindow/BP_RealityWindow.BP_RealityWindow_C|GetFrontToBackReality Entry)))))))

(fn SpawnMissingNeighbours
  (params (Room :type BP%20Room%20Object%20Reference))
  (for _array_element (Default|Doors Room)
    (if (CallFunction|IsPooledActorValid (Variables|/Game/Rooms/BP_Door.BP_Door_C|GetBackRoom _array_element))
      ;[0.15 0.15 0.15 0.5] Previous Room has been removed, flip entry to exit
      (if (not (CallFunction|IsPooledActorValid (Variables|/Game/Rooms/BP_Door.BP_Door_C|GetFrontRoom _array_element)))
        (Transformation|SetActorRotation _array_element (Math|Rotator|MakeRotator (.roll (Transformation|GetActorRotation _array_element)) (.pitch (Transformation|GetActorRotation _array_element)) (+ (.yaw (Transformation|GetActorRotation _array_element)) 1.8e+02)))
        (LocalVariables|SetFrontToBackReality (Variables|/Game/RealitySystem/RealityWindow/BP_RealityWindow.BP_RealityWindow_C|GetFrontToBackReality _array_element))
        (Variables|/Game/RealitySystem/RealityWindow/BP_RealityWindow.BP_RealityWindow_C|SetFrontToBackReality _array_element (Variables|/Game/RealitySystem/RealityWindow/BP_RealityWindow.BP_RealityWindow_C|GetBackToFrontReality _array_element))
        (Variables|/Game/RealitySystem/RealityWindow/BP_RealityWindow.BP_RealityWindow_C|SetBackToFrontReality _array_element (LocalVariables|GetFrontToBackReality))
        (Private|SpawnRoom _array_element)
        (Variables|/Game/Rooms/BP_Door.BP_Door_C|SetFrontRoom _array_element Room))
      (else
        (Private|SpawnRoom _array_element)))))

(fn NextRoomReality
  (bind _result (Math|Integer|IncrementInt (Variables|Private|GetLastRealityIndex))
    (:%20%20
      (if (> _result (- (Utilities|Array|Length (Variables|Private|GetRoomRealities)) 1))
        (Variables|Private|SetLastRealityIndex 0))
      (return (Utilities|Array|Get(acopy) (Variables|Private|GetRoomRealities) (Variables|Private|GetLastRealityIndex))))))

(fn UpdateBacktrackingOrder
  (params (Room :type BP%20Room%20Object%20Reference))
  (bind _backtrackingstack (Variables|Private|GetBacktrackingStack))
  (bind _backtrackingstack_2 (Variables|Private|GetBacktrackingStack))
  (if (Utilities|Array|ContainsItem _backtrackingstack_2 Room)
    (Utilities|Array|RemoveItem _backtrackingstack_2 Room))
  (Utilities|Array|Add _backtrackingstack_2 Room)
  (if (> (Utilities|Array|Length _backtrackingstack_2) (Variables|Default|GetBacktrackingDistance))
    (Private|RemoveRoom (Utilities|Array|Get(acopy) _backtrackingstack))
    (Utilities|Array|RemoveIndex _backtrackingstack)))

(fn RemoveRoom
  (params (Room :type BP%20Room%20Object%20Reference))
  (bind _rooms (Variables|Default|GetRooms))
  (bind _backtrackingroomids (LocalVariables|GetBacktrackingRoomIds))
  (for _array_element (Variables|Private|GetBacktrackingStack)
    (Utilities|Array|Add _backtrackingroomids (Variables|/Game/Rooms/BP_Room.BP_Room_C|GetRoomID _array_element)))
  (for _array_element_2 (Default|Doors Room)
    (bind (_containsfrontroom _containsbackroom) (Private|Helper|ContainsRoom _backtrackingroomids _array_element_2))
    (LocalVariables|SetIsFrontBacktrack _containsfrontroom)
    (LocalVariables|SetIsBackBacktrack _containsbackroom)
    ;[0.15 0.15 0.15 0.5] Remove neighbours
    (Utilities|FlowControl|Sequence
      (:then_0
        ;[0.15 0.15 0.15 0.5] Identify entry door we need to keep
        (if (and (LocalVariables|GetIsFrontBacktrack) (LocalVariables|GetIsBackBacktrack))
          (LocalVariables|SetDoorToKeep _array_element_2)))
      (:then_1
        (if (and (not (LocalVariables|GetIsFrontBacktrack)) (CallFunction|IsPooledActorValid (Variables|/Game/Rooms/BP_Door.BP_Door_C|GetFrontRoom _array_element_2)))
          (Utilities|Map|Remove _rooms (Variables|/Game/Rooms/BP_Room.BP_Room_C|GetRoomID (Variables|/Game/Rooms/BP_Door.BP_Door_C|GetFrontRoom _array_element_2)))
          (Default|RemoveRoom (Variables|/Game/Rooms/BP_Door.BP_Door_C|GetFrontRoom _array_element_2) (Utilities|Array|MakeArray _array_element_2))))
      (:then_2
        (if (and (not (LocalVariables|GetIsBackBacktrack)) (CallFunction|IsPooledActorValid (Variables|/Game/Rooms/BP_Door.BP_Door_C|GetBackRoom _array_element_2)))
          (Utilities|Map|Remove _rooms (Variables|/Game/Rooms/BP_Room.BP_Room_C|GetRoomID (Variables|/Game/Rooms/BP_Door.BP_Door_C|GetBackRoom _array_element_2)))
          (Default|RemoveRoom (Variables|/Game/Rooms/BP_Door.BP_Door_C|GetBackRoom _array_element_2) (Utilities|Array|MakeArray _array_element_2))))))
  ;[0.15 0.15 0.15 0.5] Main room to Remove
  (Utilities|Map|Remove (Variables|Default|GetRooms) (Variables|/Game/Rooms/BP_Room.BP_Room_C|GetRoomID Room))
  (Default|RemoveRoom Room (Utilities|Array|MakeArray (LocalVariables|GetDoorToKeep))))

(fn ContainsRoom
  (params (RoomIDs :type Array%20of%20Integers) (Door :type BP%20Door%20Object%20Reference))
  (bind _frontroom (Variables|/Game/Rooms/BP_Door.BP_Door_C|GetFrontRoom Door))
  (bind _backroom (Variables|/Game/Rooms/BP_Door.BP_Door_C|GetBackRoom Door))
  (Utilities|FlowControl|Sequence
    (:then_0
      (if (CallFunction|IsPooledActorValid _frontroom)
        (LocalVariables|SetFront (Utilities|Array|ContainsItem RoomIDs (Variables|/Game/Rooms/BP_Room.BP_Room_C|GetRoomID _frontroom)))))
    (:then_1
      (if (CallFunction|IsPooledActorValid _backroom)
        (LocalVariables|SetBack (Utilities|Array|ContainsItem RoomIDs (Variables|/Game/Rooms/BP_Room.BP_Room_C|GetRoomID _backroom)))))
    (:then_2
      (return (LocalVariables|GetFront) (LocalVariables|GetBack)))))

(fn InitObjectPools
  (bind _ac_roomspool (Variables|Default|GetAC_RoomsPool))
  (bind _values (Utilities|Map|Values (Variables|Private|GetExitDoorWeights)))
  (Variables|/Game/Utils/ObjectPooling/AC_ObjectPool.AC_ObjectPool_C|SetPoolSize _ac_roomspool (|((i*(n+1))+5) (.MaxValue (Math|Integer|MaxOfIntArray _values)) (Variables|Default|GetBacktrackingDistance)))
  (bind _pooledactors (Default|InitializePool _ac_roomspool))
  (for (_array_element _array_index) _pooledactors
    (bind _asbp_room (Utilities|Casting|CastToBP_Room _array_element))
    ;[0.15 0.15 0.15 0.5] Initialize rooms
    (Variables|/Game/Rooms/BP_Room.BP_Room_C|SetRoomID _asbp_room _array_index)
    (Variables|/Game/Rooms/BP_Room.BP_Room_C|SetMaxSize _asbp_room (Variables|Size|GetMax%20Size))
    (Variables|/Game/Rooms/BP_Room.BP_Room_C|SetMinSize _asbp_room (Variables|Size|GetMin%20Size))
    (Variables|/Game/Rooms/BP_Room.BP_Room_C|SetSegmentSize _asbp_room (Variables|Size|GetWallSegmentSize))
    (Variables|/Game/Rooms/BP_Room.BP_Room_C|SetExitDoorWeights _asbp_room (Variables|Private|GetExitDoorWeights))
    (Default|InitObjectPools _asbp_room)))

(fn BuildExitDoorWeightsLookup
  (bind _outrownames (DataTable|GetDataTableRowNames "/Game/Rooms/DT_ExitWeights.DT_ExitWeights"))
  (for _array_element _outrownames
    (bind _returnvalue (Utilities|GetDataTableRow "/Game/Rooms/DT_ExitWeights.DT_ExitWeights" _array_element)
      (:then
        (Utilities|Map|Add (LocalVariables|GetTempMap) (.chance _returnvalue) (.exitcount _returnvalue)))))
  ;[0.15 0.15 0.15 0.5] Calculate cummulative chances
  (bind _keys (Utilities|Map|Keys (LocalVariables|GetTempMap)))
  (for _array_element_2 _keys
    (bind _output_get (LocalVariables|SetAcummulation (+ (LocalVariables|GetAcummulation) _array_element_2)))
    (Utilities|Map|Add (Variables|Private|GetExitDoorWeights) _output_get (.Value (Utilities|Map|Find (LocalVariables|GetTempMap) _array_element_2)))))