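; Object pool component that pre-spawns actors of a configurable class for reuse.
; InitializePool destroys any existing pool and spawns PoolSize actors; it is not called from BeginPlay here.
; SpawnFromPool moves the first idle actor to a transform and flags it in use, printing a message when none is free.
; The search also collects invalid entries it passes, which RepairPool replaces with fresh spawns.
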(fn `FindFirstAvailableActor`
  (returns (PooledActor :type "/Game/Utils/ObjectPooling/BP_PooledActor Object Reference"))
  (locals (DeadObjects :type "Array of /Game/Utils/ObjectPooling/BP_PooledActor Object Reference") (FoundActor :type "/Game/Utils/ObjectPooling/BP_PooledActor Object Reference"))
  (for _array_element (`self.ObjectPool`)
    (`/Engine/EditorBlueprintResources/StandardMacros.IsValid` _array_element
      (:`Is Valid`
        (if (not (`/Game/Utils/ObjectPooling/BP_PooledActor.InUse` _array_element))
          (set `local.FoundActor` _array_element)
          (break)))
      (:`Is Not Valid`
        (`KismetArrayLibrary.Array_AddUnique` (`local.DeadObjects`) _array_element))))
  (`self.RepairPool` (`local.DeadObjects`))
  (return (`local.FoundActor`)))

(fn `InitializePool`
  (returns (PooledActors :type "Array of /Game/Utils/ObjectPooling/BP_PooledActor Object Reference"))
  (for _array_element (`self.ObjectPool`)
    (`Actor.K2_DestroyActor` _array_element))
  (for _ (range (`self.PoolSize`))
    (bind _returnvalue (`|SpawnActorFromClass` (`self.PooledActorClass`) (`KismetMathLibrary.MakeTransform` (0.0 0.0 0.0)) "Undefined" "MultiplyWithRoot" null false null))
    (`KismetArrayLibrary.Array_AddUnique` (`self.ObjectPool`) _returnvalue))
  (return (`self.ObjectPool`)))

(fn `PooledActors`
  (returns (PooledActors :type "Array of /Game/Utils/ObjectPooling/BP_PooledActor Object Reference"))
  (return (`self.ObjectPool`)))

(fn `RepairPool`
  (params (RemovedObjects :type "Array of /Game/Utils/ObjectPooling/BP_PooledActor Object Reference"))
  (bind _objectpool (`self.ObjectPool`))
  (for _array_element RemovedObjects
    (if (`KismetArrayLibrary.Array_Contains` _objectpool _array_element)
      (`KismetArrayLibrary.Array_RemoveItem` _objectpool _array_element)
      (bind _returnvalue (`|SpawnActorFromClass` (`self.PooledActorClass`) (`KismetMathLibrary.MakeTransform` (0.0 0.0 0.0)) "Undefined" "MultiplyWithRoot" null false null))
      (`KismetArrayLibrary.Array_AddUnique` (`self.ObjectPool`) _returnvalue))))

(fn `SpawnFromPool`
  (params (Transform :type "Transform Structure"))
  (returns (PooledActor :type "/Game/Utils/ObjectPooling/BP_PooledActor Object Reference"))
  (bind _pooledactor (`self.FindFirstAvailableActor`))
  (`/Engine/EditorBlueprintResources/StandardMacros.IsValid` _pooledactor
    (:`Is Valid`
      (`Actor.K2_SetActorTransform` _pooledactor Transform false false)
      (`/Game/Utils/ObjectPooling/BP_PooledActor.SetInUse` _pooledactor true)
      (return _pooledactor))
    (:`Is Not Valid`
      (`KismetSystemLibrary.PrintText` "No Actor available in Pool"))))